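; Actor component that holds a character's current main weapon and combat-enabled state.
; Setting a new main weapon unequips and destroys any valid previous one before storing the replacement.
; Toggling combat stores the flag and forwards it to the owning Character's mesh anim instance through an UpdateCombatEnabled message.
; Getters expose both the weapon and the combat state.
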(fn `GetMainWeapon`
  (returns (ReturnValue :type "/Game/CombatSystem/Blueprints/Actors/BP_BaseWeapon Object Reference"))
  (return (`self.MainWeapon`)))

(fn `IsCombatEnabled`
  (returns (ReturnValue :type Boolean))
  (return (`self.bCombatEnabled`)))

(fn `SetCombatEnabled`
  (params (bEnableCombat :type Boolean))
  (bind _output_get (set `self.bCombatEnabled` bEnableCombat))
  (message `/Game/CombatSystem/Blueprints/Interfaces/BPI_AnimInstance.UpdateCombatEnabled` (`SkeletalMeshComponent.GetAnimInstance` (`Character.Mesh` (cast `Character` (`self.GetOwner`) :!pure true))) _output_get))

(fn `SetMainWeapon`
  (params (NewWeapon :type "/Game/CombatSystem/Blueprints/Actors/BP_BaseWeapon Object Reference"))
  (bind _mainweapon (`self.MainWeapon`))
  (`|ExecutionSequence`
    (:`then_0`
      (`/Engine/EditorBlueprintResources/StandardMacros.IsValid` _mainweapon
        (:`Is Valid`
          (`/Game/CombatSystem/Blueprints/Actors/BP_BaseEquip.OnUnequip` _mainweapon)
          (`Actor.K2_DestroyActor` (`self.MainWeapon`)))))
    (:`then_1`
      (set `self.MainWeapon` (`local.NewWeapon`)))))