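; Base weapon actor in the combat system that registers itself with the main character when equipped.
; OnEquip runs the parent logic, casts the owner to BP_MainCharacter and stores itself in that character's GreatSword variable.
; The event graph holds only disabled default events, and construction just calls the parent.
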(fn `OnEquip`
  (`parent.OnEquip`)
  (bind _asbp_main_character (cast `/Game/CombatSystem/Blueprints/BP_MainCharacter` (`self.GetOwner`)))
  (set `/Game/CombatSystem/Blueprints/BP_MainCharacter.GreatSword` self _asbp_main_character))

(fn `UserConstructionScript`
  (`parent.UserConstructionScript`))